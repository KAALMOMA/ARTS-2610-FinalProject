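; Lever actor for zone 2 that, when pulled with E while the player is in range, fades in a music stem and broadcasts Lever2Activated.
; A timeline drives stem volume, lever rotation, red-to-green indicator color and MPC_Zone2 intensity.
; A watched MetaSound output also writes that intensity, making the zone's materials audio-reactive.
; The E binding is made in Tick, and the indicator's dynamic material is created on every timeline update.
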(event OnComponentBeginOverlap(collisionCube)
  (params (OverlappedComponent :type Primitive%20Component%20Object%20Reference) (OtherActor :type Actor%20Object%20Reference) (OtherComp :type Primitive%20Component%20Object%20Reference) (OtherBodyIndex :type Integer) (bFromSweep :type Boolean) (SweepResult :type Hit%20Result%20Structure%20%28by%20ref%29))
  (Variables|Default|SetplayerIsInRange true))

(event OnComponentEndOverlap(collisionCube)
  (params (OverlappedComponent :type Primitive%20Component%20Object%20Reference) (OtherActor :type Actor%20Object%20Reference) (OtherComp :type Primitive%20Component%20Object%20Reference) (OtherBodyIndex :type Integer))
  (Variables|Default|SetplayerIsInRange false))

(event Custom|pullLever
  (if (Variables|Default|GetplayerIsInRange)
    (Default|CallLever2Activated)
    (bind _alpha (Timeline|pullUpAndDown Play)
      (:Update
        (Audio|Parameter|SetFloatParameter (Variables|Default|Getmusic) "Stem2_vol" _alpha :!class /Script/Engine.AudioComponent)
        (Rendering|Material|SetScalarParameterValue "/Game/Materials/MPC_Zone2.MPC_Zone2" "MPC_intensity" (* _alpha 5.0) :!class /Script/Engine.KismetMaterialLibrary)
        (Transformation|SetRelativeRotation (Variables|Default|Getlever) (Math|Rotator|Lerp(Rotator) "0.000000,0.000000,-45.000000" "0.000000,0.000000,45.000000" _alpha) false false)
        (bind _returnvalue (Rendering|Material|CreateDynamicMaterialInstance (Variables|Default|GetindicatorBorder) 0 (Variables|Default|GetindicatorMaterial) "None" :!class /Script/Engine.PrimitiveComponent))
        (Rendering|Material|SetVectorParameterValue _returnvalue "color" (Math|Color|Lerp(LinearColor) "(R=0.068478,G=0.000000,B=0.002428,A=1.000000)" "(R=0.020289,G=0.496933,B=0.064803,A=1.000000)" _alpha) :!class /Script/Engine.MaterialInstanceDynamic)))))

(event Custom|Stem2_Amp
  (params (OutputName :type Name) (Output :type Meta%20Sound%20Output%20Structure%20%28by%20ref%29))
  (bind _returnvalue (Class|MetasoundOutputBlueprintAccess|GetFloat Output))
  (Rendering|Material|SetScalarParameterValue "/Game/Materials/MPC_Zone2.MPC_Zone2" "MPC_intensity" (+ (* _returnvalue 15.0) (* (stale Custom|pullLever _alpha) 2.0)) :!class /Script/Engine.KismetMaterialLibrary))

(event EventBeginPlay
  (Variables|Default|SetplayerIsInRange false)
  (Audio|Parameter|SetFloatParameter (Variables|Default|Getmusic) "Stem2_vol" 0.0 :!class /Script/Engine.AudioComponent)
  (MetaSoundOutput|WatchOutput (WorldSubsystems|GetMetaSoundOutputSubsystem) (Variables|Default|Getmusic) "MS_Stem2_Out" (delegate Custom|Stem2_Amp) "None" "None" :!class /Script/MetasoundEngine.MetaSoundOutputSubsystem))

(event EventTick
  (params (DeltaSeconds :type Float%20%28single-precision%29))
  (bind _asbp_side_scrolling_player_controller (Utilities|Casting|CastToBP_SideScrollingPlayerController (Game|GetPlayerController 0)))
  (EventDispatchers|BindEventtoPressE _asbp_side_scrolling_player_controller (delegate Custom|pullLever)))

(fn ConstructionScript)